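; Player controller that handles hero switching, spawning and the camera pawn used around character selection.
; The ChangeHero input asks the game instance to change character, while SpawnFunc passes the chosen class to BP_FPSGamemode to spawn or respawn the player.
; Server-named events wrap helpers that possess a new BP_Camera, reposition it and spawn the hovered character, or destroy the current pawn after saving its transform.
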(event `self.ReceiveBeginPlay`
  ;[1 1 1] Get reference to game instance at the start of play
  (bind _asbp_game_instance (cast `/Game/NewStreak/Core/GameFrameWork/BP_GameInstance` (`GameplayStatics.GetGameInstance`)))
  (set `self.GameInstanceRef` _asbp_game_instance)
  (set `self.CanRespawn` true))

(event `InputAction|Scoreboard`
  (params (Key :type "Key Structure"))
  ;[1 1 1] Scoreboard
)

(event `InputAction|ChangeHero`
  (params (Key :type "Key Structure"))
  ;[1 1 1] Change character
  (:`Pressed`
    (`/Game/NewStreak/Core/GameFrameWork/BP_GameInstance.ChangeCharacter` (`self.GameInstanceRef`) self)))

(event `SpawnFunc`
  (params (StartClass :type "/Game/NewStreak/Core/Characters/BP_FPSBaseCharacter Class Reference"))
  ;[1 1 1] Spawning via the gamemode
  (bind _asbp_fpsgamemode (cast `/Game/NewStreak/Core/GameFrameWork/BP_FPSGamemode` (`GameplayStatics.GetGameMode`)))
  (`/Game/NewStreak/Core/GameFrameWork/BP_FPSGamemode.SpawnRespawnPlayer` _asbp_fpsgamemode self StartClass))

(event `ServerSpawnCamera`
  (`self.SpawnCamera`))

(event `ServerPawnKill`
  (bind _returnvalue (`self.K2_GetPawn` self))
  (if (`KismetSystemLibrary.IsValid` _returnvalue)
    (set `self.Respawning` false)
    (set `self.CurrentPawn` (`self.GetTransform` _returnvalue))
    (`self.K2_DestroyActor` _returnvalue)
    (else
      (set `self.Respawning` true))))

(event `ServerHoveredActor`
  (params (Pawn :type "Pawn Object Reference") (SelectedCharacter :type "/Game/NewStreak/Core/Characters/BP_FPSBaseCharacter Class Reference"))
  (`self.HoverActor` self Pawn SelectedCharacter))

(fn `HoverActor`
  (params (Pawn :type "Pawn Object Reference") (Class :type "Actor Class Reference"))
  (returns (SpawnedActor :type "Actor Object Reference"))
  (bind (_asbp_camera _bsuccess) (cast `/Game/NewStreak/Maps/CharacterSelect/BP_Camera` Pawn :!pure true))
  (`KismetSystemLibrary.PrintString` (`KismetStringLibrary.Conv_BoolToString` _bsuccess))
  (`self.K2_SetActorLocation` _asbp_camera (`self.StandardLocation`) true false)
  (bind _returnvalue (`|SpawnActorFromClass` Class (`self.SpawnActorLocation`) "AlwaysSpawn" "OverrideRootScale" null null))
  (set `self.SpawnedActor` _returnvalue)
  (return _returnvalue))

(fn `SpawnCamera`
  (bind _returnvalue (`|SpawnActorFromClass` "/Game/NewStreak/Maps/CharacterSelect/BP_Camera.BP_Camera_C" (`self.OffsetTrans`) "Undefined" "OverrideRootScale" self null))
  (`self.Possess` self _returnvalue))

(fn `UserConstructionScript`)