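; Hitscan weapon Blueprint that fires instant line traces from the owner's camera toward the crosshair.
; OnFire and BeginFire re-trigger each other through a FireRate-gated timer, with semi-automatic weapons ending after one shot.
; Authority runs spread-cone traces, spawns first- and third-person tracers, and applies ammo-based point damage with impact effects.
; Character hits show a hitmarker or killmarker, predicted from pre-damage health, and call RecoverFuelDistortion on the shooter.
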(event `self.ReceiveBeginPlay`
  (bind _returnvalue (`AddComponent|NODE_AddBP_BaseAmmo-0`))
  (set `self.CurrentAmmoType` _returnvalue))

(event `self.OnFire`
  (params (CrosshairWorldSpace :type "Vector Structure"))
  (bind _crosshairworldspace (`/Game/NewStreak/Core/Characters/BP_FPSBaseCharacter.GetCrosshairWorldSpace` (`self.OwningCharacter`)))
  (`parent.OnFire` _crosshairworldspace)
  (if (`self.CanFire?`)
    (`self.ServerDetermineHit` _crosshairworldspace)
    (`self.BeginFire`)))

(event `self.BeginFire`
  (bind _lastfired (`self.LastFired`))
  (`parent.BeginFire`)
  (bind _output_get (set `self.GameTime` (`GameplayStatics.GetTimeSeconds`)))
  (if (> _lastfired 0.0)
    (if (>= (- _output_get _lastfired) (`self.FireRate`))
      (`self.CallOnFire` :!label _label)
      (else
        (`KismetSystemLibrary.K2_SetTimer` null "CallOnFire" (- (+ (`self.LastFired`) (`self.FireRate`)) (`self.GameTime`)))))
    (else
      (goto _label))))

(event `self.EndFire`
  (`parent.EndFire`)
  (`KismetSystemLibrary.K2_ClearTimer` null "CallOnFire"))

(event `ServerDetermineHit`
  (params (CrosshairWorldSpace :type "Vector Structure"))
  (`self.DetermineHitObjects` CrosshairWorldSpace))

(event `ServerImpactEffects`
  (params (HitLocation :type "Vector Structure"))
  (`self.PlayImpactEffects` HitLocation))

(event `ClientHitmarker`
  (`GameplayStatics.PlaySound2D` "/Game/NewStreak/Assets/SoundEffects/HitmarkerSoundBak.HitmarkerSoundBak" 1.0 1.0 0.0 null null)
  (bind _returnvalue (`|CreateWidget` "/Game/NewStreak/Core/CoreUIandEffects/WBP_Hitmarker.WBP_Hitmarker_C"))
  (`UserWidget.AddToViewport` _returnvalue 0))

(event `Killmarker`
  (`GameplayStatics.PlaySound2D` "/Game/NewStreak/Assets/SoundEffects/HitmarkerSoundBak.HitmarkerSoundBak" 1.0 1.0 0.0 null null)
  (bind _returnvalue (`|CreateWidget` "/Game/NewStreak/Core/CoreUIandEffects/WBP_Hitmarker.WBP_Hitmarker_C"))
  (`UserWidget.AddToViewport` _returnvalue 0))

(fn `ApplyDamageToHitActors`
  (locals (`ShowHitmarker?` :type Boolean) (HitCharacter :type "/Game/NewStreak/Core/Characters/BP_FPSBaseCharacter Object Reference") (HealthBeforeDamage :type "Float (double-precision)" :default 0.0))
  (bind _returnvalue (`self.GetInstigatorController`))
  (bind _hitresult (`self.HitResult`))
  (bind (_bblockinghit _binitialoverlap _time _distance _location _impactpoint _normal _impactnormal _physmat _hitactor) (`GameplayStatics.BreakHitResult` _hitresult))
  (`/Engine/EditorBlueprintResources/ActorMacros.Switch Has Authority`
    (:`Authority`
      (bind _asbp_fpsbase_character (cast `/Game/NewStreak/Core/Characters/BP_FPSBaseCharacter` _hitactor)
        (:`then`
          (bind _output_get (set `local.HitCharacter` _asbp_fpsbase_character))
          (set `local.HealthBeforeDamage` (`/Game/NewStreak/Core/Characters/BP_FPSBaseCharacter.Health` _output_get))
          (set `local.ShowHitmarker?` true))
        (:`CastFailed`
          (set `local.ShowHitmarker?` false)))
      (`GameplayStatics.ApplyPointDamage` _hitactor (`/Game/NewStreak/Core/Weapons/BP_BaseAmmo.BaseDamage` (`self.CurrentAmmoType`)) (`KismetMathLibrary.Conv_RotatorToVector` (`KismetMathLibrary.FindLookAtRotation` _location (`self.K2_GetActorLocation` (`Controller.K2_GetPawn` _returnvalue)))) _hitresult _returnvalue self)
      (bind _output_get_2 (set `self.HitLocation` _location))
      (`self.ServerImpactEffects` _output_get_2)
      (if (`local.ShowHitmarker?`)
        (if (<= (- (`local.HealthBeforeDamage`) (`/Game/NewStreak/Core/Weapons/BP_BaseAmmo.BaseDamage` (`self.CurrentAmmoType`))) 0.0)
          (`self.Killmarker`)
          (else
            (`self.ClientHitmarker`)))
        (`/Game/NewStreak/Core/Characters/BP_FPSBaseCharacter.RecoverFuelDistortion` (`self.OwningCharacter`))
        (set `self.HitResult` (struct))))))

(fn `CallOnFire`
  (`self.OnFire` (0.0 0.0 0.0))
  (if (not (`self.AutomaticFire?`))
    (set `/Game/NewStreak/Core/Characters/BP_FPSBaseCharacter.Firing?` false (`self.OwningCharacter`))
    (`self.EndFire`)))

(fn `DetermineHitObjects`
  (params (CrosshairWorldSpace :type "Vector Structure"))
  (returns (`HitOccured?` :type Boolean))
  (locals (`ObjectHit?` :type Boolean))
  (bind _returnvalue (`SceneComponent.GetSocketLocation` (`self.Mesh`) (`self.MuzzleSocket`)))
  (bind _returnvalue_2 (`SceneComponent.K2_GetComponentLocation` (`/Game/NewStreak/Core/Characters/BP_FPSBaseCharacter.FirstPersonCamera` (`self.OwningCharacter`))))
  (bind _returnvalue_3 (* (`KismetMathLibrary.RandomUnitVectorInConeInRadians` (1.0 0.0 0.0) (`KismetMathLibrary.DegreesToRadians` (`self.Spread`))) (`self.Range`)))
  (bind _returnvalue_4 (`KismetMathLibrary.GreaterGreater_VectorRotator` _returnvalue_3 (`KismetMathLibrary.FindLookAtRotation` _returnvalue_2 CrosshairWorldSpace)))
  (`/Engine/EditorBlueprintResources/ActorMacros.Switch Has Authority`
    (:`Authority`
      (set `self.HitResult` (struct))
      (for _ (range 1 (+ (`self.TracesUsed`) 1))
        (bind (_outhit _returnvalue_5) (`KismetSystemLibrary.LineTraceSingle` _returnvalue_2 (+ _returnvalue_2 _returnvalue_4) "TraceTypeQuery1" false (`|MakeArray` (`self.Instigator`) :!type "Actor Object Reference")))
        (bind _output_get (set `local.ObjectHit?` (or _returnvalue_5 (`local.ObjectHit?`))))
        (if _output_get
          (set `self.HitResult` _outhit)
          (else
            (set `self.HitResult` (struct))))
        (`self.SpawnTracer` CrosshairWorldSpace _returnvalue_3 _returnvalue (- (+ _returnvalue _returnvalue_4) _returnvalue) (`local.ObjectHit?`))
        (if _output_get
          (`self.ApplyDamageToHitActors`)))
      (return (`local.ObjectHit?`)))))

(fn `PlayImpactEffects`
  (params (Location :type "Vector Structure"))
  (`GameplayStatics.SpawnEmitterAtLocation` (`self.HitImpactEffects`) Location (`KismetMathLibrary.Conv_VectorToRotator` Location) (0.1 0.1 0.1)))

(fn `SpawnTracer`
  (params (CroshaiirWorldPosition :type "Vector Structure") (RandomUnitVector :type "Vector Structure") (SocketLocation :type "Vector Structure") (RortationFromX :type "Vector Structure") (HitOccured :type Boolean))
  (locals (EndOfTrace :type "Transform Structure") (EndOfTrace3p :type "Transform Structure"))
  (bind _returnvalue (`self.GetOwner`))
  (bind (_bblockinghit _binitialoverlap _time _distance _location) (`GameplayStatics.BreakHitResult` (`self.HitResult`)))
  (bind _returnvalue_2 (`SceneComponent.GetSocketLocation` (`/Game/NewStreak/Core/Characters/BP_FPSBaseCharacter.FP_Gun` (`self.OwningCharacter`)) (`self.MuzzleSocket`)))
  (if HitOccured
    (set `local.EndOfTrace` (`KismetMathLibrary.MakeTransform` SocketLocation (`KismetMathLibrary.Conv_VectorToRotator` (- _location SocketLocation))))
    (else
      (set `local.EndOfTrace` (`KismetMathLibrary.MakeTransform` SocketLocation (`KismetMathLibrary.Conv_VectorToRotator` RortationFromX)))))
  (`|SpawnActorFromClass` (`self.Tracer1P`) (`local.EndOfTrace`) "Undefined" "OverrideRootScale" _returnvalue null) ; FirstPerson Tracer
  (if true
    (set `local.EndOfTrace3p` (`KismetMathLibrary.MakeTransform` _returnvalue_2 (`KismetMathLibrary.Conv_VectorToRotator` (- _location _returnvalue_2))))
    (else
      (set `local.EndOfTrace3p` (`KismetMathLibrary.MakeTransform` _returnvalue_2 (`KismetMathLibrary.Conv_VectorToRotator` (- (+ _returnvalue_2 (`KismetMathLibrary.GreaterGreater_VectorRotator` RandomUnitVector (`KismetMathLibrary.FindLookAtRotation` _returnvalue_2 CroshaiirWorldPosition))) _returnvalue_2))))))
  (`|SpawnActorFromClass` (`self.Tracer3P`) (`local.EndOfTrace3p`) "Undefined" "OverrideRootScale" _returnvalue null) ; ThirdPersonTracer
)

(fn `UserConstructionScript`
  (`parent.UserConstructionScript`))