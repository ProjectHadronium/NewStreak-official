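; Menu showcase Blueprint that displays two different, randomly chosen characters on its left and right skeletal meshes.
; On BeginPlay it rolls two random indices and rerolls both until they differ.
; Each index then selects one of seven character meshes, from Assassin to Wraith, and applies it to its side with the pose reinitialized.
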(event `self.ReceiveBeginPlay`
  (`self.RNGSwitch` :!label _label)
  (`self.RNGSwitch1`)
  (if (== (`self.Switch`) (`self.Switch1`))
    (goto _label)
    (else
      (`|ExecutionSequence`
        (:`then_0`
          (switch `int` (`self.Switch`)
            (:`0`
              (set `self.TheChosen` "/Game/NewStreak/Blueprints/Characters/Assassin/SK_Assassin.SK_Assassin"))
            (:`1`
              (set `self.TheChosen` "/Game/NewStreak/Blueprints/Characters/Enforcer/SK_Enforcer.SK_Enforcer"))
            (:`2`
              (set `self.TheChosen` "/Game/NewStreak/Blueprints/Characters/Gunslinger/SK_Gunslinger.SK_Gunslinger"))
            (:`3`
              (set `self.TheChosen` "/Game/NewStreak/Blueprints/Characters/Harrier/SK_Harrier.SK_Harrier"))
            (:`4`
              (set `self.TheChosen` "/Game/NewStreak/Blueprints/Characters/Juggernaut/SK_Juggs.SK_Juggs"))
            (:`5`
              (set `self.TheChosen` "/Game/NewStreak/Blueprints/Characters/Vanguard/SK_Vanguard.SK_Vanguard"))
            (:`6`
              (set `self.TheChosen` "/Game/NewStreak/Blueprints/Characters/Wraith/SK_Wraith.SK_Wraith")))
          (`SkinnedMeshComponent.SetSkinnedAssetAndUpdate` (`self.MeshRight`) (`self.TheChosen`) true))
        (:`then_1`
          (switch `int` (`self.Switch1`)
            (:`0`
              (set `self.TheSecondChosen` "/Game/NewStreak/Blueprints/Characters/Assassin/SK_Assassin.SK_Assassin"))
            (:`1`
              (set `self.TheSecondChosen` "/Game/NewStreak/Blueprints/Characters/Enforcer/SK_Enforcer.SK_Enforcer"))
            (:`2`
              (set `self.TheSecondChosen` "/Game/NewStreak/Blueprints/Characters/Gunslinger/SK_Gunslinger.SK_Gunslinger"))
            (:`3`
              (set `self.TheSecondChosen` "/Game/NewStreak/Blueprints/Characters/Harrier/SK_Harrier.SK_Harrier"))
            (:`4`
              (set `self.TheSecondChosen` "/Game/NewStreak/Blueprints/Characters/Juggernaut/SK_Juggs.SK_Juggs"))
            (:`5`
              (set `self.TheSecondChosen` "/Game/NewStreak/Blueprints/Characters/Vanguard/SK_Vanguard.SK_Vanguard"))
            (:`6`
              (set `self.TheSecondChosen` "/Game/NewStreak/Blueprints/Characters/Wraith/SK_Wraith.SK_Wraith")))
          (`SkinnedMeshComponent.SetSkinnedAssetAndUpdate` (`self.MeshLeft`) (`self.TheSecondChosen`) true))))))

(fn `RNGSwitch`
  (set `self.Switch` (`KismetMathLibrary.RandomInteger` 7)))

(fn `RNGSwitch1`
  (set `self.Switch1` (`KismetMathLibrary.RandomInteger` 7)))

(fn `UserConstructionScript`)