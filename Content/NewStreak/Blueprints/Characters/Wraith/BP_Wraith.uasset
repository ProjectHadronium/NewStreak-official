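; Wraith player character with a pip-limited mid-air "warp jump" alongside its normal jump, plus a pip HUD widget.
; An airborne jump capsule-traces along the stored jump direction; a hit gives a free wall jump along input or the mirrored bounce.
; A miss spends a pip to launch along input plus scaled current velocity.
; A timeline blends into the new velocity, and landing starts a looping timer that refills pips while not falling.
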(event `self.ReceiveBeginPlay`
  ;[1 1 1] BeginPlay
  (`parent.ReceiveBeginPlay`)
  (bind _returnvalue (`|CreateWidget` "/Game/NewStreak/Core/CoreUIandEffects/BP_Pips.BP_Pips_C"))
  (`UserWidget.AddToViewport` _returnvalue 0))

(event `self.OnLanded`
  (params (Hit :type "HitResult Structure (by ref)"))
  ;[1 1 1] Landed
  (`self.RegenTimer`))

(event `InputAction|MoveAbility`
  (params (Key :type "Key Structure"))
  ;[1 1 1] MoveAbility
)

(event `InputAction|Jump`
  (params (Key :type "Key Structure"))
  ;[1 1 1] WJ
  (:`Pressed`
    (`self.WJ`)))

(event `WJ`
  ;[1 1 1] WJ
  (if (`CharacterMovementComponent.IsWalking` (`self.CharacterMovement`))
    (`self.BaseJump` (0.0 0.0 750.0))
    (set `self.WJDirection` (`self.GetLastMovementInputVector`))
    (else
      (`self.ServerWJCapsuleTrace`)
      (if (`self.CapsuleTraceHit`)
        (if (`self.InputCheck`)
          (`self.WJWindDown` (`self.WJMultiplier`))
          (else
            (`self.WJWindDown` (`self.MirrorVelocity`))))
        (elif (> (`self.Pips`) 0)
          (`self.WJWindDown` (+ (`self.WJMultiplier`) (* (`MovementComponent.Velocity` (`self.CharacterMovement`)) (`self.WJScale`))))
          (`self.ServerCountPip`)))
      (set `self.WJDirection` (`MovementComponent.Velocity` (`self.CharacterMovement`))))))

(event `RegenTimer`
  ;[1 1 1] WJ
  (bind _returnvalue (`KismetSystemLibrary.K2_SetTimerDelegate` (delegate `PipRegen`) 0.25 true)))

(event `PipRegen`
  ;[1 1 1] WJ
  (`self.PipRegenFunc` (stale `RegenTimer` _returnvalue)))

(event `ServerWJCapsuleTrace`
  ;[1 1 1] WJ
  (`self.WJCapsuleTrace`))

(event `WJWindDown`
  (params (InputVelocity :type "Vector Structure"))
  ;[1 1 1] WJ
  (`self.WindDown` InputVelocity))

(event `ServerCountPip`
  ;[1 1 1] WJ
  (set `self.Pips` (- (`self.Pips`) 1)))

(fn `CountPip`
  (set `self.Pips` (- (`self.Pips`) 1)))

(fn `PipRegenFunc`
  (params (TimerHandle :type "TimerHandle Structure"))
  (if (not (`NavMovementComponent.IsFalling` (`self.CharacterMovement`)))
    (set `self.Pips` (+ (`self.Pips`) 1))
    (if (not (< (`self.Pips`) (`self.TotalPips`)))
      (`KismetSystemLibrary.K2_ClearAndInvalidateTimerHandle` TimerHandle))))

(fn `UserConstructionScript`
  (`parent.UserConstructionScript`))

(fn `WJCapsuleTrace`
  (bind _returnvalue (`SceneComponent.K2_GetComponentLocation` (`self.FirstPersonCamera`)))
  (bind (_returnvalue_x _returnvalue_y) (`KismetMathLibrary.BreakVector` (`KismetMathLibrary.Normal` (`self.WJDirection`))))
  (bind _returnvalue_2 (+ _returnvalue (* (`KismetMathLibrary.MakeVector` _returnvalue_x _returnvalue_y) (`self.LTLength`))))
  (bind (_outhit _returnvalue_3) (`KismetSystemLibrary.CapsuleTraceSingle` :`Start` _returnvalue :`End` _returnvalue_2 :`Radius` 65.0 :`HalfHeight` 122.0 :`TraceChannel` "TraceTypeQuery2" :`DrawDebugType` "ForDuration"))
  (set `self.CapsuleTraceHit` _returnvalue_3)
  (set `self.MirrorVelocity` (* (`KismetMathLibrary.MakeVector` (.x (`KismetMathLibrary.Normal` (`KismetMathLibrary.MirrorVectorByNormal` (- _returnvalue_2 _returnvalue) (`.ImpactNormal` (`GameplayStatics.BreakHitResult` _outhit))))) (.y (`KismetMathLibrary.Normal` (`KismetMathLibrary.MirrorVectorByNormal` (- _returnvalue_2 _returnvalue) (`.ImpactNormal` (`GameplayStatics.BreakHitResult` _outhit))))) (`self.ZScale`)) (`self.WarpJumpMultiplier`))))

(fn `WJVelocityLerp`
  (params (EndVelocity :type "Vector Structure") (Alpha :type "Float (double-precision)"))
  (bind _charactermovement (`self.CharacterMovement`))
  (set `MovementComponent.Velocity` (`KismetMathLibrary.VLerp` (`MovementComponent.Velocity` _charactermovement) EndVelocity Alpha) _charactermovement))