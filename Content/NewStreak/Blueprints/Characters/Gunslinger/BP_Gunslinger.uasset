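; Gunslinger player character with a pip-limited dash (warp), an airborne warp jump, and a thrown knife projectile.
; Input events call Server-named events for dash and knife, while warp jump runs from local input; Ultimate and Blindfire are empty stubs.
; Warps use timelines to lerp velocity up and down with camera shake, then spend a pip and start looping regen timers.
; Knife cooldown destroys the projectile, but its TacKnifed gate is never set true here.
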(event `self.ReceiveBeginPlay`
  ;[1 1 1] BeginPlay
  (`parent.ReceiveBeginPlay`)
  (bind _returnvalue (`|CreateWidget` "/Game/NewStreak/Core/CoreUIandEffects/BP_DashPips.BP_DashPips_C"))
  (`UserWidget.AddToViewport` _returnvalue 0))

(event `InputAction|MoveAbility`
  (params (Key :type "Key Structure"))
  (bind (_returnvalue_roll _returnvalue_pitch _returnvalue_yaw) (`KismetMathLibrary.BreakRotator` (`SceneComponent.K2_GetComponentRotation` (`self.FirstPersonCamera`))))
  (bind _returnvalue (`PawnMovementComponent.GetLastInputVector` (`self.CharacterMovement`)))
  ;[1 1 1] InputEvents
  (:`Pressed`
    (set `self.WarpInput` _returnvalue)
    (`KismetSystemLibrary.PrintString` (`KismetStringLibrary.Conv_VectorToString` _returnvalue))
    (set `self.Direction1` (`KismetMathLibrary.GetForwardVector` (`KismetMathLibrary.MakeRotator` 0.0 _returnvalue_pitch _returnvalue_yaw)))
    (`self.ServerMoveAbility` (`self.WarpInput`) (`self.Direction1`))))

(event `ServerTacKnife`
  (bind _firstpersoncamera (`self.FirstPersonCamera`))
  ;[1 1 1] AbilityServerEvents
  (if (not (`self.TacKnifed`))
    (set `self.TacKnifed` false)
    (bind _returnvalue (`|SpawnActorFromClass` "/Game/NewStreak/Blueprints/Characters/Gunslinger/BP_GSProjectile.BP_GSProjectile_C" (`KismetMathLibrary.MakeTransform` (+ (`SceneComponent.K2_GetComponentLocation` _firstpersoncamera) (* (`SceneComponent.GetForwardVector` _firstpersoncamera) 170.0)) (`self.GetControlRotation`) (0.5 0.5 0.5)) "AlwaysSpawn" "OverrideRootScale" null (`GameplayStatics.GetPlayerCharacter` 0)))
    (if (`self.TacKnifed`)
      (bind _returnvalue_2 (`KismetSystemLibrary.K2_SetTimerDelegate` (delegate `TacRegenTimer`) 0.1 true)))))

(event `TacRegenTimer`
  ;[1 1 1] AbilityServerEvents
  (`self.ServerTacCooldown` (stale `ServerTacKnife` _returnvalue_2) (stale `ServerTacKnife` _returnvalue)))

(event `InputAction|Jump`
  (params (Key :type "Key Structure"))
  ;[1 1 1] InputEvents
  (:`Pressed`
    (if (`CharacterMovementComponent.IsWalking` (`self.CharacterMovement`))
      (`self.Jump`)
      (else
        (`self.JumpEvent`)))))

(event `JumpEvent`
  (bind _warpjumpresetspeed (`self.WarpJumpResetSpeed`))
  (bind _charactermovement (`self.CharacterMovement`))
  ;[1 1 1] AbilityServerEvents
  (if (> (`self.Pips`) 0)
    (set `self.WarpJumpFinalSpeed` (* (`self.WarpJumpInput`) (`self.WarpJumpMultiplier`)))
    (set `self.WarpJumpResetSpeed` (`MovementComponent.Velocity` (`self.CharacterMovement`)))
    (`CharacterMovementComponent.AddImpulse` (`self.CharacterMovement`) (0.0 0.0 50.0) true)
    (bind (_direction _warpwindup) (`Timeline|WarpJumpInitial` :!via `PlayFromStart`)
      (:`Update`
        (set `MovementComponent.Velocity` (+ (`KismetMathLibrary.VLerp` (`self.WarpJumpResetSpeed`) (`self.WarpJumpFinalSpeed`) _warpwindup) (`MovementComponent.Velocity` _charactermovement)) _charactermovement))
      (:`Finished`
        (`GameplayStatics.PlayWorldCameraShake` "/Game/NewStreak/Core/CoreUIandEffects/BP_WarpShake.BP_WarpShake_C" (`self.K2_GetActorLocation`) 0.0 500.0)
        (set `self.WarpJumpResetSpeed` (`MovementComponent.Velocity` (`self.CharacterMovement`)))
        (bind (_direction_2 _warp) (`Timeline|WarpJumpSlowDown` :!via `PlayFromStart`)
          (:`Update`
            (set `MovementComponent.Velocity` (`KismetMathLibrary.VLerp` _warpjumpresetspeed (* _warpjumpresetspeed (`self.WarpJumpWindDown`)) _warp) (`self.CharacterMovement`)))
          (:`Finished`
            (`self.ServerCountPip`)
            (if (not (`self.WarpCooldownActive`))
              (bind _returnvalue (`KismetSystemLibrary.K2_SetTimerDelegate` (delegate `Regen`) 0.0225 true))
              (set `self.WarpCooldownActive` true))))))))

(event `Regen`
  ;[1 1 1] AbilityServerEvents
  (`self.ServerPipCooldown` (stale `JumpEvent` _returnvalue)))

(event `ServerMoveAbility`
  (params (InputVector :type "Vector Structure") (Dir1 :type "Vector Structure"))
  (bind _returnvalue (`KismetMathLibrary.VSize` InputVector))
  (bind _warpresetspeed (`self.WarpResetSpeed`))
  (bind _charactermovement (`self.CharacterMovement`))
  ;[1 1 1] AbilityServerEvents
  (if (> (`self.Pips`) 0)
    (`KismetSystemLibrary.PrintString` (`KismetStringLibrary.Conv_DoubleToString` _returnvalue))
    (if (!= _returnvalue 0.0)
      (set `self.WarpFinalSpeed` (* InputVector (`self.WarpMultiplier`)))
      (else
        (set `self.WarpFinalSpeed` (* Dir1 (`self.WarpMultiplier`)))))
    (set `self.WarpResetSpeed` (`MovementComponent.Velocity` _charactermovement))
    (`CharacterMovementComponent.AddImpulse` _charactermovement (0.0 0.0 50.0) true)
    (bind (_direction _warpwindup) (`Timeline|WarpInitial` :!via `PlayFromStart`)
      (:`Update`
        (set `MovementComponent.Velocity` (`KismetMathLibrary.VLerp` (`self.WarpResetSpeed`) (`self.WarpFinalSpeed`) _warpwindup) (`self.CharacterMovement`)))
      (:`Finished`
        (`GameplayStatics.PlayWorldCameraShake` "/Game/NewStreak/Core/CoreUIandEffects/BP_WarpShake.BP_WarpShake_C" (`self.K2_GetActorLocation`) 0.0 500.0)
        (set `self.WarpResetSpeed` (`MovementComponent.Velocity` (`self.CharacterMovement`)))
        (bind (_direction_2 _warp) (`Timeline|WarpSlowDown` :!via `PlayFromStart`)
          (:`Update`
            (set `MovementComponent.Velocity` (`KismetMathLibrary.VLerp` _warpresetspeed (* _warpresetspeed (`self.WarpWindDown`)) _warp) (`self.CharacterMovement`)))
          (:`Finished`
            (`self.ServerCountPip`)
            (if (not (`self.WarpCooldownActive`))
              (bind _returnvalue_2 (`KismetSystemLibrary.K2_SetTimerDelegate` (delegate `WPipRegen`) 0.0225 true))
              (set `self.WarpCooldownActive` true))))))))

(event `WPipRegen`
  ;[1 1 1] AbilityServerEvents
  (`self.ServerPipCooldown` (stale `ServerMoveAbility` _returnvalue_2)))

(event `ServerTacCooldown`
  (params (Handle :type "TimerHandle Structure") (ReturnValue :type "/Game/NewStreak/Blueprints/Characters/Gunslinger/BP_GSProjectile Object Reference"))
  ;[1 1 1] Replication Events
  (`self.TacCooldown` Handle ReturnValue))

(event `InputAction|Ability2`
  (params (Key :type "Key Structure"))
  ;[1 1 1] InputEvents
  (:`Pressed`
    (`self.ServerTacKnife`)))

(event `ServerBlindFire`
  ;[1 1 1] AbilityServerEvents
)

(event `ServerPipCooldown`
  (params (Handle :type "TimerHandle Structure"))
  ;[1 1 1] Replication Events
  (`self.PipCooldown` Handle))

(event `InputAction|Blindfire`
  (params (Key :type "Key Structure"))
  ;[1 1 1] InputEvents
  (:`Pressed`
    (`self.ServerBlindFire`)))

(event `ServerUltimate`
  ;[1 1 1] AbilityServerEvents
)

(event `ServerCountPip`
  ;[1 1 1] Replication Events
  (`self.CountPip`))

(event `InputAction|Ability1`
  (params (Key :type "Key Structure"))
  ;[1 1 1] InputEvents
  (:`Pressed`
    (`self.ServerUltimate`)))

(fn `UserConstructionScript`
  (`parent.UserConstructionScript`))