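; BP_GravityVolume is a box volume that changes a BP_FPSBaseCharacter's gravity according to its height inside the box.
; Overlap starts a roughly 60 Hz looping timer that passes the new scale to the character's GravityField, skipped during distortion or grappling.
; Construction caches the box's vertical bounds, and the scale steps from zero in the lower portion up to partial gravity near the top.
; End overlap only clears the timer; the gravity reset logic is disconnected.
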(event `GravTimer`
  (bind (_asbp_fpsbase_character _bsuccess) (cast `/Game/NewStreak/Core/Characters/BP_FPSBaseCharacter` (stale `self.Box.OnComponentBeginOverlap` OtherActor) :!pure true))
  (if (`/Game/NewStreak/Core/Characters/BP_FPSBaseCharacter.DistortionActive?` _asbp_fpsbase_character)
    _
    (elif (not (`/Game/NewStreak/Core/Characters/BP_FPSBaseCharacter.Grappling?` _asbp_fpsbase_character))
      (bind (_returnvalue_x _returnvalue_y _returnvalue_z) (`KismetMathLibrary.BreakVector` (`self.K2_GetActorLocation` _asbp_fpsbase_character)))
      (bind _newgravscale (`self.CaculateNewGravityScale` _returnvalue_z))
      (`/Game/NewStreak/Core/Characters/BP_FPSBaseCharacter.GravityField` _asbp_fpsbase_character _newgravscale))))

(event `self.Box.OnComponentBeginOverlap`
  (params (OverlappedComponent :type "PrimitiveComponent Object Reference") (OtherActor :type "Actor Object Reference") (OtherComp :type "PrimitiveComponent Object Reference") (OtherBodyIndex :type Integer) (bFromSweep :type Boolean) (SweepResult :type "HitResult Structure (by ref)"))
  (if (`.bSuccess` (cast `/Game/NewStreak/Core/Characters/BP_FPSBaseCharacter` OtherActor :!pure true))
    (bind _returnvalue (`KismetSystemLibrary.K2_SetTimer` null "GravTimer" 0.01667 true))))

(event `self.Box.OnComponentEndOverlap`
  (params (OverlappedComponent :type "PrimitiveComponent Object Reference") (OtherActor :type "Actor Object Reference") (OtherComp :type "PrimitiveComponent Object Reference") (OtherBodyIndex :type Integer))
  (`KismetSystemLibrary.K2_ClearAndInvalidateTimerHandle` (stale `self.Box.OnComponentBeginOverlap` _returnvalue)))

(fn `CaculateNewGravityScale`
  (params (ActorLocation :type "Float (double-precision)"))
  (returns (NewGravScale :type "Float (double-precision)"))
  (locals (PercentageHeight :type "Float (double-precision)" :default 0.0) (NewGravityScale :type "Float (double-precision)"))
  (bind _percentageheight (`local.PercentageHeight`))
  (set `local.PercentageHeight` (/ (- ActorLocation (`self.FloorLocation`)) (`self.Height`)))
  (if (> _percentageheight 0.9)
    (set `local.NewGravityScale` 0.4)
    (elif (> _percentageheight 0.8)
      (set `local.NewGravityScale` 0.3)
      (elif (> _percentageheight 0.7)
        (set `local.NewGravityScale` 0.2)
        (elif (> _percentageheight 0.6)
          (set `local.NewGravityScale` 0.1)
          (else
            (set `local.NewGravityScale` 0.0))))))
  (return (`local.NewGravityScale`)))

(fn `UserConstructionScript`
  (bind (_origin _boxextent) (`KismetSystemLibrary.GetComponentBounds` (`self.Box`)))
  (bind _output_get (set `self.CentreLocation` (.z _origin)))
  (bind _output_get_2 (set `self.TopLocation` (+ (.z _origin) (.z _boxextent))))
  (set `self.FloorLocation` (- _output_get (- _output_get_2 _output_get)))
  (set `self.Height` (- (`self.TopLocation`) (`self.FloorLocation`))))